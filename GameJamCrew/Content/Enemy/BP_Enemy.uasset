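; Chef enemy that patrols random locations, investigates sounds and hunts the player, ending the match with a restart menu on contact within its view cone.
; An integer state machine drives AIMoveTo through patrol, alert pause, chase, nearby search and capture, switching animations and player music.
; Tick-based sight checks feed transitions, combining distance, angle limits and head-socket traces to the player's head, then tail.
; It manually yaws toward movement or the visible player.
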(event `self.ReceiveBeginPlay`
  ;[1 1 1] Find a reference to the player
  (bind _returnvalue (`GameplayStatics.GetActorOfClass` "/Game/ThirdPersonBP/Blueprints/ThirdPersonCharacter.ThirdPersonCharacter_C" :!label _label))
  (`/Engine/EditorBlueprintResources/StandardMacros.IsValid` _returnvalue
    (:`Is Valid`
      (set `self.ChaseTarget` _returnvalue)
      (`self.State 0`))
    (:`Is Not Valid`
      (`KismetSystemLibrary.Delay` 0.2)
      (goto _label))))

(event `self.ReceiveTick`
  (params (DeltaSeconds :type "Float (single-precision)"))
  (bind _returnvalue (`self.GetVelocity`))
  (bind _visible (`self.CheckVisibility`))
  (set `self.TargetVisible` _visible)
  (if (>= (`KismetMathLibrary.VSize` _returnvalue) 0.1)
    (`self.RotateToTarget` (+ (`self.K2_GetActorLocation` self) _returnvalue))
    (elif (`self.TargetVisible`)
      (`self.RotateToTarget` (`self.K2_GetActorLocation` (`self.ChaseTarget`)))))
  (if (and (`self.TargetVisible`) (<= (`self.State`) 0))
    (`self.ChangeState` 1)))

(event `ChangeState`
  (params (NewState :type Integer))
  (bind _chasetarget (`self.ChaseTarget`))
  (bind _output_get (set `self.State` NewState))
  (switch `int` _output_get
    (:`0`
      (`self.State 0`)
      (`/Game/ThirdPersonBP/Blueprints/ThirdPersonCharacter.UpdateMusic` _chasetarget 1))
    (:`1`
      (`self.State 1`)
      (`GameplayStatics.PlaySound2D` "/Game/audio/ost/highIntensity_intro.highIntensity_intro" 1.0 1.0 0.0 null null)
      (`/Game/ThirdPersonBP/Blueprints/ThirdPersonCharacter.UpdateVolume` (`self.ChaseTarget`) 0.5))
    (:`2`
      (`self.State 2`)
      (`/Game/ThirdPersonBP/Blueprints/ThirdPersonCharacter.UpdateMusic` _chasetarget 3))
    (:`3`
      (`self.State 3`))
    (:`4`
      (`self.State 4`)
      (`/Game/ThirdPersonBP/Blueprints/ThirdPersonCharacter.UpdateMusic` _chasetarget 4))))

(event `UpdateAnim`
  (params (Type :type Integer))
  (bind _skeletalmesh (`self.SkeletalMesh`))
  (if (!= Type (`self.CurrentAnim`))
    (bind _output_get (set `self.CurrentAnim` Type))
    (switch `int` _output_get
      (:`0`
        (`SkeletalMeshComponent.PlayAnimation` _skeletalmesh "/Game/Enemy/Chef/A_ChefIdle.A_ChefIdle" true))
      (:`1`
        (`SkeletalMeshComponent.PlayAnimation` _skeletalmesh "/Game/Enemy/Chef/A_ChefWalk.A_ChefWalk" true))
      (:`2`
        (`SkeletalMeshComponent.PlayAnimation` _skeletalmesh "/Game/Enemy/Chef/A_ChefKneelDown.A_ChefKneelDown" false)))))

(event `State 0`
  (bind _output (`|GetArrayItem` (`self.RandomLocations`) (`KismetMathLibrary.RandomIntegerInRange` 0 (- (`KismetArrayLibrary.Array_Length` (`self.RandomLocations`)) 1))))
  (if (<= (`KismetMathLibrary.VSize` (- (`self.K2_GetActorLocation`) _output)) 10.0)
    (`self.State 0`)
    (else
      (`|AIMoveTo` self _output null
        (:`then`
          (`self.UpdateAnim` 1))
        (:`OnSuccess`
          (`self.UpdateAnim` 0 :!label _label_2)
          (`KismetSystemLibrary.Delay` (`KismetMathLibrary.RandomFloatInRange` 1.5 3.0))
          (if (== (`self.State`) 0)
            (`self.State 0`)))
        (:`OnFail`
          (goto _label_2))))))

(event `InvestigateSound`
  (params (Location :type "Vector Structure"))
  (if (not (`self.TargetVisible`))
    (set `self.State` -1)
    (`|AIMoveTo` self Location null 25.0
      (:`OnSuccess`
        _)
      (:`OnFail`
        _))
    (`self.UpdateAnim` 0)
    (if (not (`self.TargetVisible`))
      (`self.ChangeState` 0))))

(event `State 1`
  (`|AIMoveTo` self (`self.K2_GetActorLocation`) null 25.0
    (:`then`
      (`self.UpdateAnim` 0)
      (`KismetSystemLibrary.Delay` 3.0)
      (if (`self.TargetVisible`)
        (`self.ChangeState` 2)
        (else
          (`self.ChangeState` 0))))))

(event `State 2`
  (`|AIMoveTo` self (`self.K2_GetActorLocation` (`self.ChaseTarget`)) null 25.0
    (:`then`
      (`self.UpdateAnim` 1)
      (`KismetSystemLibrary.Delay` 1.0)
      (if (== (`self.State`) 2)
        (if (`self.TargetVisible`)
          (`self.State 2`))))
    (:`OnSuccess`
      (if (== (`self.State`) 2) :!label _label_3
        (if (`self.TargetVisible`)
          (`self.State 2`)
          (else
            (`self.ChangeState` 3)))))
    (:`OnFail`
      (goto _label_3))))

(event `State 3`
  (`|AIMoveTo` self (+ (`self.K2_GetActorLocation`) (* (`KismetMathLibrary.RandomUnitVector`) (250.0 250.0 0.0))) null 25.0
    (:`then`
      (`self.UpdateAnim` 1))
    (:`OnSuccess`
      (`self.UpdateAnim` 0 :!label _label_4)
      (if (== (`self.State`) 3)
        (if (`self.TargetVisible`)
          (`self.ChangeState` 2)
          (else
            (`KismetSystemLibrary.Delay` 2.0)
            (if (== (`self.State`) 3)
              (`self.ChangeState` 0))))))
    (:`OnFail`
      (goto _label_4))))

(event `State 4`
  (`MovementComponent.StopMovementImmediately` (`self.FloatingPawnMovement`))
  (`self.UpdateAnim` 2)
  (`/Game/ThirdPersonBP/Blueprints/ThirdPersonCharacter.EndMatch` (`self.ChaseTarget`))
  (bind _returnvalue (`|CreateWidget` "/Game/ThirdPersonBP/Blueprints/UI_MenuRestart.UI_MenuRestart_C" (`GameplayStatics.GetPlayerController` 0)))
  (bind _output_get (set `self.WidgetRef` _returnvalue))
  (`UserWidget.AddToViewport` _output_get 0)
  (`/Game/ThirdPersonBP/Blueprints/UI_MenuRestart.UpdateMission` _output_get false))

(event `self.Capsule.OnComponentBeginOverlap`
  (params (OverlappedComponent :type "PrimitiveComponent Object Reference") (OtherActor :type "Actor Object Reference") (OtherComp :type "PrimitiveComponent Object Reference") (OtherBodyIndex :type Integer) (bFromSweep :type Boolean) (SweepResult :type "HitResult Structure (by ref)"))
  (if (== OtherActor (`self.ChaseTarget`))
    (if (`self.InLOS`)
      (`self.ChangeState` 4))))

(event `FootstepSound`
  (bind _returnvalue (`KismetMathLibrary.RandomFloatInRange` 0.8 1.2))
  (`GameplayStatics.PlaySoundAtLocation` (`|GetArrayItem` (`self.FootstepSounds`) (`KismetMathLibrary.RandomIntegerInRange` 0 5)) (`self.K2_GetActorLocation`) (struct) _returnvalue _returnvalue 0.0 null null null))

(fn `CheckVisibility`
  (returns (Visible :type Boolean))
  (bind _losangle (`self.LOSAngle`))
  (bind _losangle_2 (`self.LOSAngle`))
  (bind (_returnvalue_roll _returnvalue_pitch _returnvalue_yaw) (`KismetMathLibrary.BreakRotator` (`KismetMathLibrary.NormalizedDeltaRotator` (`self.K2_GetActorRotation` self) (`KismetMathLibrary.FindLookAtRotation` (`self.K2_GetActorLocation` self) (`self.K2_GetActorLocation` (`self.ChaseTarget`))))))
  (if (<= (`KismetMathLibrary.Vector_Distance` (`self.K2_GetActorLocation` self) (`self.K2_GetActorLocation` (`self.ChaseTarget`))) (`self.VisibleDistance`))
    (bind _output_get (set `self.InLOS` (and (`KismetMathLibrary.InRange_FloatFloat` _returnvalue_roll (* _losangle -1.0) _losangle) (`KismetMathLibrary.InRange_FloatFloat` _returnvalue_pitch -75.0 75.0) (`KismetMathLibrary.InRange_FloatFloat` (+ _returnvalue_yaw 90.0) (* _losangle_2 -1.0) _losangle_2))))
    (if _output_get
      (bind (_outhit _returnvalue) (`KismetSystemLibrary.LineTraceSingle` :`Start` (`SceneComponent.GetSocketLocation` (`self.SkeletalMesh`) "CC_Base_Head") :`End` (`SceneComponent.GetSocketLocation` (`Character.Mesh` (`self.ChaseTarget`)) "Head3") :`TraceChannel` "TraceTypeQuery1" :`DrawDebugType` "ForOneFrame" :`DrawTime` 0.0))
      (if _returnvalue
        (if (== (`.HitActor` (`GameplayStatics.BreakHitResult` _outhit)) (`self.ChaseTarget`))
          (return true)
          (else
            _)))
      (bind (_outhit_2 _returnvalue_2) (`KismetSystemLibrary.LineTraceSingle` :`Start` (`SceneComponent.GetSocketLocation` (`self.SkeletalMesh`) "CC_Base_Head") :`End` (`SceneComponent.GetSocketLocation` (`Character.Mesh` (`self.ChaseTarget`)) "Tail3") :`TraceChannel` "TraceTypeQuery1" :`DrawDebugType` "ForOneFrame" :`DrawTime` 0.0))
      (if _returnvalue_2
        (return (== (`.HitActor` (`GameplayStatics.BreakHitResult` _outhit_2)) (`self.ChaseTarget`)))
        (else
          (return false)))
      (else
        (return false)))
    (else
      (return false))))

(fn `RotateToTarget`
  (params (Target :type "Vector Structure (by ref)"))
  (bind (_returnvalue_roll _returnvalue_pitch) (`KismetMathLibrary.BreakRotator` (`self.K2_GetActorRotation`)))
  (bind (_returnvalue_roll_2 _returnvalue_pitch_2 _returnvalue_yaw) (`KismetMathLibrary.BreakRotator` (`KismetMathLibrary.FindLookAtRotation` (`self.K2_GetActorLocation` self) Target)))
  (`self.K2_SetActorRotation` (`KismetMathLibrary.MakeRotator` _returnvalue_roll _returnvalue_pitch (- _returnvalue_yaw 90.0)) true))

(fn `UserConstructionScript`)